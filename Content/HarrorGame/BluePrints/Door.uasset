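; Interactive door Blueprint that swings open and closed when the E key is pressed, with no proximity check.
; A FlipFlop alternates between playing and reversing the SmoothKapi timeline, setting a play rate and playing an open or close sound at the door.
; Opening captures the root's world rotation and a target 90 degrees further in yaw, and the timeline lerps the root between them.
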(event `Key|E`
  (params (Key :type "Key Structure"))
  (bind _returnvalue (`SceneComponent.K2_GetComponentLocation` (`self.Door`)))
  (bind _returnvalue_2 (`SceneComponent.K2_GetComponentRotation` (`self.DefaultSceneRoot`)))
  (:`Pressed`
    (`/Engine/EditorBlueprintResources/StandardMacros.FlipFlop`
      (:`A`
        (set `self.BaseRotation` _returnvalue_2)
        (set `self.TargetRotation` (`KismetMathLibrary.MakeRotator` (.roll _returnvalue_2) (.pitch _returnvalue_2) (+ (.yaw _returnvalue_2) 90.0)))
        (`TimelineComponent.SetPlayRate` 0.4)
        (`GameplayStatics.PlaySoundAtLocation` "/Game/HarrorGame/Sesler/doorOpen.doorOpen" _returnvalue (struct) 1.0 1.0 0.0 null null null)
        (bind (_direction _kapimovement) (`Timeline|SmoothKapi` :!label _label)
          (:`Update`
            (`SceneComponent.K2_SetWorldRotation` (`self.DefaultSceneRoot`) (`KismetMathLibrary.RLerp` (`self.BaseRotation`) (`self.TargetRotation`) _kapimovement) false false))))
      (:`B`
        (`TimelineComponent.SetPlayRate` (`self.SmoothKapi`) 0.9)
        (`GameplayStatics.PlaySoundAtLocation` "/Game/HarrorGame/Sesler/doorClose.doorClose" _returnvalue (struct) 1.0 1.0 0.0 null null null)
        (goto _label :!via `Reverse`)))))

(fn `UserConstructionScript`)